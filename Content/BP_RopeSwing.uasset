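; Rope swing actor that lets the player grab, swing on and jump from a referenced cable actor.
; Overlapping its box enables input; holding F attaches the player to the CableEnd socket at their current height and disables character movement.
; W and S set opposing world-X cable forces, which are never reset.
; Releasing F detaches the player, restores falling, launches them forward and up, and disables the actor's input.
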(event `self.Box.OnComponentBeginOverlap`
  (params (OverlappedComponent :type "PrimitiveComponent Object Reference") (OtherActor :type "Actor Object Reference") (OtherComp :type "PrimitiveComponent Object Reference") (OtherBodyIndex :type Integer) (bFromSweep :type Boolean) (SweepResult :type "HitResult Structure (by ref)"))
  (`self.EnableInput` self (`GameplayStatics.GetPlayerController` 0)))

(event `Key|F`
  (params (Key :type "Key Structure"))
  (bind _returnvalue (`GameplayStatics.GetPlayerCharacter` 0))
  (bind (_returnvalue_x _returnvalue_y) (`KismetMathLibrary.BreakVector` (`self.K2_GetActorLocation` _returnvalue)))
  (bind (_returnvalue_x_2 _returnvalue_y_2 _returnvalue_z) (`KismetMathLibrary.BreakVector` (`self.K2_GetActorLocation` (`GameplayStatics.GetPlayerCharacter` 0))))
  (bind _charactermovement (`Character.CharacterMovement` _returnvalue))
  (:`Pressed`
    (set `self.PlayerHeight` _returnvalue_z)
    (`self.K2_AttachToActor` _returnvalue (`self.CableRef`) "CableEnd" "SnapToTarget" "KeepWorld" "KeepWorld" true)
    (`self.K2_SetActorLocation` _returnvalue (`KismetMathLibrary.MakeVector` _returnvalue_x _returnvalue_y (`self.PlayerHeight`)) false false)
    (`CharacterMovementComponent.SetMovementMode` _charactermovement "MOVE_None" 0))
  (:`Released`
    (`self.K2_DetachFromActor` _returnvalue "KeepWorld" "KeepWorld" "KeepWorld")
    (`CharacterMovementComponent.SetMovementMode` _charactermovement "MOVE_Falling" 0)
    (`Character.LaunchCharacter` _returnvalue (+ (* (`self.GetActorForwardVector` _returnvalue) 1000.0) (* (`self.GetActorUpVector` _returnvalue) 400.0)) false false)
    (`self.DisableInput` self (`GameplayStatics.GetPlayerController` 0))))

(event `Key|W`
  (params (Key :type "Key Structure"))
  (:`Pressed`
    (set `CableComponent.CableForce` (100.0 0.0 0.0) (`CableActor.CableComponent` (`self.CableRef`)))))

(event `Key|S`
  (params (Key :type "Key Structure"))
  (:`Pressed`
    (set `CableComponent.CableForce` (-100.0 0.0 0.0) (`CableActor.CableComponent` (`self.CableRef`)))))

(fn `UserConstructionScript`)
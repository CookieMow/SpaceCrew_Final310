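; BP_LightLever is a puzzle lever that switches an array of affected lights on and off.
; BeginPlay applies the initial IsOn state to each light's root visibility.
; LeverMoving plays a switch sound, inverts IsOn and updates the lights, while a timeline lerps the lever's rotation forward or back.
; The timeline's FlipFlop fires inside each light loop, so it toggles once per light rather than once per pull.
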(event `self.ReceiveBeginPlay`
  (for _array_element (`self.AffectedLights`)
    (`SceneComponent.SetVisibility` (`Actor.RootComponent` _array_element) (`self.IsOn`) false)))

(event `LeverMoving`
  (`GameplayStatics.PlaySoundAtLocation` "/Engine/VREditor/Sounds/UI/Flashlight_Switch.Flashlight_Switch" (`self.K2_GetActorLocation`) (struct) 1.0 1.0 0.0 null null null null)
  (bind _output_get (set `self.IsOn` (not (`self.IsOn`))))
  (if _output_get
    (for _array_element (`self.AffectedLights`)
      (`SceneComponent.SetVisibility` (`Actor.RootComponent` _array_element) true false)
      (`/Engine/EditorBlueprintResources/StandardMacros.FlipFlop` :!label _label
        (:`A`
          (bind (_direction _alpha) (`Timeline|moving up and down` :!label _label_2)
            (:`Update`
              (`SceneComponent.K2_SetRelativeRotation` (`self.lever`) (`KismetMathLibrary.RLerp` (struct :`Roll` -40.0) (struct :`Roll` -140.0) _alpha) false false))))
        (:`B`
          (goto _label_2 :!via `Reverse`))))
    (else
      (for _array_element_2 (`self.AffectedLights`)
        (`SceneComponent.SetVisibility` (`Actor.RootComponent` _array_element_2) false false)
        (goto _label)))))

(fn `UserConstructionScript`)
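; BP_Lever is a puzzle lever that toggles on and off, playing a switch sound each time its LeverMoving event fires.
; Each toggle increments or decrements SwitchCount on the referenced BP_puzzleManager, then calls its UpdateSwitchCount.
; A FlipFlop then alternately plays and reverses the MovingUpAndDown timeline, which lerps the lever's relative rotation between two positions.
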(event `LeverMoving`
  (`GameplayStatics.PlaySoundAtLocation` "/Engine/VREditor/Sounds/UI/Flashlight_Switch.Flashlight_Switch" (`self.K2_GetActorLocation`) (struct) 1.0 1.0 0.0 null null null null)
  (bind _output_get (set `self.IsOn` (not (`self.IsOn`))))
  (if _output_get
    (bind _asbp_puzzle_manager (cast `/Game/Puzzle/BP_puzzleManager` (`self.Manager`)))
    (set `/Game/Puzzle/BP_puzzleManager.SwitchCount` (+ (`/Game/Puzzle/BP_puzzleManager.SwitchCount` _asbp_puzzle_manager) 1) _asbp_puzzle_manager)
    (else
      (bind _asbp_puzzle_manager_2 (cast `/Game/Puzzle/BP_puzzleManager` (`self.Manager`)))
      (set `/Game/Puzzle/BP_puzzleManager.SwitchCount` (- (`/Game/Puzzle/BP_puzzleManager.SwitchCount` _asbp_puzzle_manager_2) 1) _asbp_puzzle_manager_2)))
  (`/Game/Puzzle/BP_puzzleManager.UpdateSwitchCount` _asbp_puzzle_manager_2)
  (`/Game/Puzzle/BP_puzzleManager.UpdateSwitchCount` _asbp_puzzle_manager)
  (`/Engine/EditorBlueprintResources/StandardMacros.FlipFlop`
    (:`A`
      (bind (_direction _alpha) (`Timeline|moving up and down` :!label _label)
        (:`Update`
          (`SceneComponent.K2_SetRelativeRotation` (`self.lever`) (`KismetMathLibrary.RLerp` (struct :`Pitch` -40.0) (struct :`Pitch` -120.0) _alpha) false false))))
    (:`B`
      (goto _label :!via `Reverse`))))

(fn `UserConstructionScript`)
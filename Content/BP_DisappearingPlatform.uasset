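; Disappearing platform that warns the player, then vanishes after they step on it.
; A player character entering the Box trigger swaps the Floor material and runs timed sounds, then hides the Floor and disables its collision after about two seconds.
; Any end overlap restores material, visibility and collision after a one-second delay, without cancelling a pending disappearance.
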(event `self.Box.OnComponentBeginOverlap`
  (params (OverlappedComponent :type "PrimitiveComponent Object Reference") (OtherActor :type "Actor Object Reference") (OtherComp :type "PrimitiveComponent Object Reference") (OtherBodyIndex :type Integer) (bFromSweep :type Boolean) (SweepResult :type "HitResult Structure (by ref)"))
  (cast `/Game/ThirdPerson/Blueprints/BP_ThirdPersonCharacter1` OtherActor)
  (`GameplayStatics.PlaySound2D` "/Game/Audio/blockBreak6_33.blockBreak6_33" 1.0 1.0 0.0 null null)
  (`PrimitiveComponent.SetMaterial` (`self.floor`) 0 "/Engine/MapTemplates/Materials/BasicAsset01.BasicAsset01")
  (`KismetSystemLibrary.Delay` 1.0)
  (`GameplayStatics.PlaySound2D` "/Game/Audio/blocked_30.blocked_30" 1.0 1.0 0.0 null null)
  (`KismetSystemLibrary.Delay` 1.0)
  (`SceneComponent.SetVisibility` (`self.floor`) false false)
  (`GameplayStatics.PlaySound2D` "/Game/Audio/blockBreak_27.blockBreak_27" 1.0 1.0 0.0 null null)
  (`PrimitiveComponent.SetCollisionEnabled` (`self.floor`) "NoCollision"))

(event `self.Box.OnComponentEndOverlap`
  (params (OverlappedComponent :type "PrimitiveComponent Object Reference") (OtherActor :type "Actor Object Reference") (OtherComp :type "PrimitiveComponent Object Reference") (OtherBodyIndex :type Integer))
  (`KismetSystemLibrary.Delay` 1.0)
  (`PrimitiveComponent.SetMaterial` (`self.floor`) 0 "/Game/BaseMaterial.BaseMaterial")
  (`SceneComponent.SetVisibility` (`self.floor`) true false)
  (`PrimitiveComponent.SetCollisionEnabled` (`self.floor`) "QueryAndPhysics"))

(fn `UserConstructionScript`)
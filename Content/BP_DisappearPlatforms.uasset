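; Platform actor that disappears shortly after the third-person player character steps on it, then reappears after they leave.
; Box begin overlap, filtered to BP_ThirdPersonCharacter, swaps Floor to an Xray material as a warning, then after a delay hides it and disables collision.
; Box end overlap, unfiltered by actor, waits briefly before resetting the material slot and restoring visibility and collision.
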(event `self.Box.OnComponentBeginOverlap`
  (params (OverlappedComponent :type "PrimitiveComponent Object Reference") (OtherActor :type "Actor Object Reference") (OtherComp :type "PrimitiveComponent Object Reference") (OtherBodyIndex :type Integer) (bFromSweep :type Boolean) (SweepResult :type "HitResult Structure (by ref)"))
  (cast `/Game/ThirdPerson/Blueprints/BP_ThirdPersonCharacter` OtherActor)
  (`PrimitiveComponent.SetMaterial` (`self.Floor`) 0 "/Engine/VREditor/TransformGizmo/Xray.Xray")
  (`KismetSystemLibrary.Delay` 1.0)
  (`SceneComponent.SetVisibility` (`self.Floor`) false false)
  (`PrimitiveComponent.SetCollisionEnabled` (`self.Floor`) "NoCollision"))

(event `self.Box.OnComponentEndOverlap`
  (params (OverlappedComponent :type "PrimitiveComponent Object Reference") (OtherActor :type "Actor Object Reference") (OtherComp :type "PrimitiveComponent Object Reference") (OtherBodyIndex :type Integer))
  (`KismetSystemLibrary.Delay` 2.0)
  (`PrimitiveComponent.SetMaterial` (`self.Floor`) 0 null)
  (`SceneComponent.SetVisibility` (`self.Floor`) true false)
  (`PrimitiveComponent.SetCollisionEnabled` (`self.Floor`) "QueryAndPhysics"))

(fn `UserConstructionScript`)